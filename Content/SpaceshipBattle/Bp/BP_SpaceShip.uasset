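; BP_SpaceShip is the spaceship Blueprint for the SpaceshipBattle game, adding a console toggle and a screen-fade function.
; The Console input action flips the ShowConsole flag on AircraWarsGameModeBase.
; The Start function adds a Fade widget to the viewport, plays its animation slowly in reverse and returns it, though nothing in this file calls it.
; BeginPlay, Tick, overlap and the construction script are empty.
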(event EventBeginPlay)

(event Collision|EventActorBeginOverlap
  (params (OtherActor :type Actor%20Object%20Reference)))

(event EventTick
  (params (DeltaSeconds :type Float%20%28single-precision%29)))

(event Input|ActionEvents|InputActionConsole
  (params (Key :type Key%20Structure :default "None"))
  (:Pressed
    (bind _asaircra_wars_game_mode_base (Utilities|Casting|CastToAircraWarsGameModeBase (Game|GetGameMode)))
    (if (Variables|/Script/AircraWar.AircraWarsGameModeBase|GetShowConsole _asaircra_wars_game_mode_base)
      (Variables|/Script/AircraWar.AircraWarsGameModeBase|SetShowConsole _asaircra_wars_game_mode_base false)
      (else
        (Variables|/Script/AircraWar.AircraWarsGameModeBase|SetShowConsole _asaircra_wars_game_mode_base true)))))

(fn ConstructionScript)

(fn Start
  (bind _returnvalue (UserInterface|CreateWidget "/Game/SpaceshipBattle/HUD/Fade.Fade_C"))
  (UserInterface|Viewport|AddtoViewport _returnvalue 0)
  (UserInterface|Animation|PlayAnimation _returnvalue (Variables|/Game/SpaceshipBattle/HUD/Fade.Fade_C|GetFade _returnvalue) 0.0 1 "Reverse" 0.2 false)
  (return _returnvalue))